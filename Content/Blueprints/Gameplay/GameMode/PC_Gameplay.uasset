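; PC_Gameplay is the gameplay player controller, handling gender-based player spawning, push-to-talk voice chat and a server-full notice.
; ClientHandleGender reads IsMale from GI_Main and passes it to ServerRequestGender, which asks GM_Gameplay to spawn this controller's player.
; The VOIP input action starts voice chat on press and stops it on release.
; ShowServerFull creates the WBP_ServerFull widget and adds it to the viewport.
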(event `ServerRequestGender`
  (params (IsMale :type Boolean))
  (bind _asgm_gameplay (cast `/Game/Blueprints/Gameplay/GameMode/GM_Gameplay` (`GameplayStatics.GetGameMode`)))
  (`/Game/Blueprints/Gameplay/GameMode/GM_Gameplay.SpawnPC` _asgm_gameplay self IsMale))

(event `ClientHandleGender`
  (bind _asgi_main (cast `/Game/Blueprints/General/GI_Main` (`GameplayStatics.GetGameInstance`)))
  (`self.ServerRequestGender` (`/Game/Blueprints/General/GI_Main.IsMale` _asgi_main)))

(event `InputAction|VOIP`
  (params (Key :type "Key Structure"))
  (:`Pressed`
    (`UniversalVoiceChat.VoiceChatStartSpeak` true))
  (:`Released`
    (`UniversalVoiceChat.VoiceChatStopSpeak`)))

(event `ShowServerFull`
  (bind _returnvalue (`|CreateWidget` "/Game/Widgets/WBP_ServerFull.WBP_ServerFull_C"))
  (`UserWidget.AddToViewport` _returnvalue 0))

(fn `UserConstructionScript`)