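; Gameplay game mode that admits players up to a limit and spawns their gendered character.
; On login it tracks each PC_Gameplay and triggers its gender handling, or shows a server-full notice; logout removes it from the list.
; SpawnPC, after a short delay, spawns an actor with VOIP attenuation and a male or female character at a random cached PlayerStart, then possesses the character.
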(event `SpawnPC`
  (params (PC :type "/Game/Blueprints/Gameplay/GameMode/PC_Gameplay Object Reference") (IsMale :type Boolean))
  (bind (_spawntransform_location _spawntransform_rotation) (`KismetMathLibrary.BreakTransform` (`self.GetPlayerStart`)))
  (`KismetSystemLibrary.Delay` 0.2)
  (`|SpawnActorFromClass` "/Script/UniversalVoiceChatPro.PlayerVoiceChatActor" (`KismetMathLibrary.MakeTransform` (0.0 0.0 0.0)) "Undefined" "OverrideRootScale" PC 0 "/Game/Audio/SA_VOIP.SA_VOIP" false true true 1000.0 null)
  (bind _returnvalue (`|SpawnActorFromClass` (select `bool` IsMale :`false` "/Game/Blueprints/Gameplay/GameMode/BP_Character_Female.BP_Character_Female_C" :`true` "/Game/Blueprints/Gameplay/GameMode/BP_Character_Male.BP_Character_Male_C" :!type "Actor Class Reference") (`KismetMathLibrary.MakeTransform` _spawntransform_location _spawntransform_rotation) "Undefined" "OverrideRootScale" PC null))
  (bind _aspawn (cast `Pawn` _returnvalue))
  (`Controller.Possess` PC _aspawn))

(event `self.ReceiveBeginPlay`
  (bind _outactors (`GameplayStatics.GetAllActorsOfClass` "/Script/Engine.PlayerStart"))
  (set `self.PlayerStarts` _outactors))

(event `self.K2_PostLogin`
  (params (NewPlayer :type "PlayerController Object Reference"))
  (bind _aspc_gameplay (cast `/Game/Blueprints/Gameplay/GameMode/PC_Gameplay` NewPlayer))
  (`self.CheckCanJoin`
    (:`CanJoin`
      (`KismetArrayLibrary.Array_Add` (`self.PCs`) _aspc_gameplay)
      (`/Game/Blueprints/Gameplay/GameMode/PC_Gameplay.ClientHandleGender` _aspc_gameplay))
    (:`CannotJoin`
      (`/Game/Blueprints/Gameplay/GameMode/PC_Gameplay.ShowServerFull` _aspc_gameplay))))

(event `self.K2_OnLogout`
  (params (ExitingController :type "Controller Object Reference"))
  (bind _aspc_gameplay (cast `/Game/Blueprints/Gameplay/GameMode/PC_Gameplay` ExitingController))
  (`KismetArrayLibrary.Array_RemoveItem` (`self.PCs`) _aspc_gameplay))

(fn `GetPlayerStart`
  (returns (SpawnTransform :type "Transform Structure"))
  (bind _playerstarts (`self.PlayerStarts`))
  (return (`self.GetTransform` (`|GetArrayItem` _playerstarts (`KismetMathLibrary.RandomIntegerInRange` 0 (`KismetArrayLibrary.Array_LastIndex` _playerstarts))))))

(fn `UserConstructionScript`)